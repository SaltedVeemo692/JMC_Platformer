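; BP_Player_Bullet is a player projectile actor that moves itself and expires after a set lifetime.
; Each Tick lerps Speed toward zero by SpeedDamp, then applies a non-swept local offset along the normalized Trejectory vector.
; Movement and damping are per frame, without delta-time scaling.
; The same Tick chain runs a LifeTime Delay before destroying the actor; the graph contains no hit or damage logic.
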(event `self.ReceiveTick`
  (params (DeltaSeconds :type "Float (single-precision)"))
  ; Bullet movement
  (set `self.Speed` (`KismetMathLibrary.Lerp` (`self.Speed`) 0.0 (`self.SpeedDamp`)))
  (`self.K2_AddActorLocalOffset` (* (`KismetMathLibrary.Normal` (`self.Trejectory`)) (`self.Speed`)))
  (`KismetSystemLibrary.Delay` (`self.LifeTime`))
  (`self.K2_DestroyActor`))

(fn `UserConstructionScript`)