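; BP_NPC is a non-player character that shows an interact prompt and plays a sequence of dialogue lines.
; Its trigger zone toggles the prompt's visibility when the cached BP_ThirdPersonCharacter player enters or leaves.
; StartDialogue resets the line index and calls UpdateDialogue, which writes each line into the player's CurrentDialogueText.
; UpdateDialogue re-calls itself after a fixed delay, clearing the text after the last line.
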(event `self.ReceiveBeginPlay`
  (bind _asbp_third_person_character (cast `/Game/ThirdPerson/Blueprints/BP_ThirdPersonCharacter` (`GameplayStatics.GetPlayerPawn` 0)))
  (set `self.PlayerReference` _asbp_third_person_character))

(event `self.C_NPCTriggerZone.OnComponentBeginOverlap`
  (params (OverlappedComponent :type "PrimitiveComponent Object Reference") (OtherActor :type "Actor Object Reference") (OtherComp :type "PrimitiveComponent Object Reference") (OtherBodyIndex :type Integer) (bFromSweep :type Boolean) (SweepResult :type "HitResult Structure (by ref)"))
  ; Show Interact button
  (if (== OtherActor (`self.PlayerReference`))
    (`SceneComponent.SetVisibility` (`self.Interact_Prompt`) true false)))

(event `self.C_NPCTriggerZone.OnComponentEndOverlap`
  (params (OverlappedComponent :type "PrimitiveComponent Object Reference") (OtherActor :type "Actor Object Reference") (OtherComp :type "PrimitiveComponent Object Reference") (OtherBodyIndex :type Integer))
  ; Show Interact button
  (if (== OtherActor (`self.PlayerReference`))
    (`SceneComponent.SetVisibility` (`self.Interact_Prompt`) false false)))

(event `UpdateDialogue`
  (set `/Game/ThirdPerson/Blueprints/BP_ThirdPersonCharacter.CurrentDialogueText` (`|GetArrayItem` (`self.DialogueLines`) (`self.CurrentDialogueLine`)) (`self.PlayerReference`))
  (bind _output_get (set `self.CurrentDialogueLine` (+ (`self.CurrentDialogueLine`) 1)))
  (`KismetSystemLibrary.Delay` 2.0)
  (if (!= _output_get (`KismetArrayLibrary.Array_Length` (`self.DialogueLines`)))
    (`self.UpdateDialogue`)
    (else
      (set `/Game/ThirdPerson/Blueprints/BP_ThirdPersonCharacter.CurrentDialogueText` "" (`self.PlayerReference`)))))

(event `StartDialogue`
  (set `self.CurrentDialogueLine` 0)
  (`self.UpdateDialogue`))

(fn `UserConstructionScript`)