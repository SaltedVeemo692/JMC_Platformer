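; A platform that vanishes after the player has stood on it, then reappears after a delay.
; Player overlap with the trigger zone starts a Tick-driven timer that keeps running after they leave, jumping ahead to a cutoff if they step off earlier.
; When the timer reaches the lifetime, the actor hides and disables collision, then restores its starting transform, visibility and collision after the invisible period.
; Debug prints show contact and elapsed time.
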(event `self.ReceiveBeginPlay`
  (set `self.StartTransform` (`self.GetTransform`)))

(event `self.TriggerZone.OnComponentBeginOverlap`
  (params (OverlappedComponent :type "PrimitiveComponent Object Reference") (OtherActor :type "Actor Object Reference") (OtherComp :type "PrimitiveComponent Object Reference") (OtherBodyIndex :type Integer) (bFromSweep :type Boolean) (SweepResult :type "HitResult Structure (by ref)"))
  ; On and Off platforms
  (if (== OtherActor (`GameplayStatics.GetPlayerPawn` 0))
    (`|ExecutionSequence`
      (:`then_0`
        (`KismetSystemLibrary.PrintString` "PLAYER ON PLATFORM"))
      (:`then_1`
        (set `self.IsPlayerOnPlatform` true)))))

(event `self.TriggerZone.OnComponentEndOverlap`
  (params (OverlappedComponent :type "PrimitiveComponent Object Reference") (OtherActor :type "Actor Object Reference") (OtherComp :type "PrimitiveComponent Object Reference") (OtherBodyIndex :type Integer))
  ; On and Off platforms
  (if (and (== OtherActor (`GameplayStatics.GetPlayerPawn` 0)) (< (`self.TimeOnPlatform`) (`self.TimeOnPlatformCutOff`)))
    (set `self.TimeOnPlatform` (`self.TimeOnPlatformCutOff`))))

(event `self.ReceiveTick`
  (params (DeltaSeconds :type "Float (single-precision)"))
  ; Tick platform time
  (if (`self.IsPlayerOnPlatform`)
    (bind _output_get (set `self.TimeOnPlatform` (+ (`self.TimeOnPlatform`) DeltaSeconds)))
    (`|ExecutionSequence`
      (:`then_0`
        ; CHECK PLATFORM END OF LIFE
        (if (>= (`self.TimeOnPlatform`) (`self.PlatformLifeTime`))
          ; platform end of life
          (`self.SetActorHiddenInGame` true)
          (`self.SetActorEnableCollision` false)
          (set `self.IsPlayerOnPlatform` false)
          (`KismetSystemLibrary.Delay` (`self.TimeInvisible`))
          (`self.ReturnToStart`)))
      (:`then_1`
        (`KismetSystemLibrary.PrintString` (`KismetStringLibrary.Conv_DoubleToString` _output_get))))
    (else
      (set `self.TimeOnPlatform` 0.0))))

(event `ReturnToStart`
  ; respawn function
  (`SceneComponent.K2_SetWorldTransform` (`self.DefaultSceneRoot`) (`self.StartTransform`) false true)
  (set `self.TimeOnPlatform` 0.0)
  (`self.SetActorHiddenInGame` false)
  (`self.SetActorEnableCollision` true))

(fn `UserConstructionScript`)