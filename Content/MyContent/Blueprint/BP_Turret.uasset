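; Turret actor that continuously fires BP_Bullet projectiles and can optionally rotate its body to face the player.
; BeginPlay picks single-shot or scatter-shot mode via UseScatterShot, and each mode loops by calling itself after FiringDelay.
; Bullets spawn at FiringPoint, with scatter shots firing a burst with randomized pitch and yaw.
; When LookAtPlayer is set, Tick sets SMTurretBody's relative rotation using only X/Y positions.
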(event `self.ReceiveBeginPlay`
  ; Initiate shots
  (if (`self.UseScatterShot`)
    (`self.ScatterShot`)
    (else
      (`self.OneShot`))))

(event `self.ReceiveTick`
  (params (DeltaSeconds :type "Float (single-precision)"))
  (bind (_returnvalue_x _returnvalue_y) (`KismetMathLibrary.BreakVector` (`self.K2_GetActorLocation`)))
  (bind (_returnvalue_x_2 _returnvalue_y_2) (`KismetMathLibrary.BreakVector` (`self.K2_GetActorLocation` (`GameplayStatics.GetPlayerPawn` 0))))
  ; Rotate towards player
  (if (`self.LookAtPlayer`)
    (`SceneComponent.K2_SetRelativeRotation` (`self.SM_Turret_Body`) (`KismetMathLibrary.FindLookAtRotation` (`KismetMathLibrary.MakeVector` _returnvalue_x _returnvalue_y) (`KismetMathLibrary.MakeVector` _returnvalue_x_2 _returnvalue_y_2)) false false)))

(event `ScatterShot`
  (bind _returnvalue (`SceneComponent.GetSocketTransform` (`self.FiringPoint`) "None" "RTS_World"))
  ; scatter shot
  (for _ (range 5)
    (`|SpawnActorFromClass` "/Game/MyContent/Blueprint/BP_Bullet.BP_Bullet_C" (`KismetMathLibrary.MakeTransform` (.location _returnvalue) (`KismetMathLibrary.MakeRotator` (.roll (.rotation _returnvalue)) (+ (.pitch (.rotation _returnvalue)) (`KismetMathLibrary.RandomFloatInRange` -30.0 30.0)) (+ (.yaw (.rotation _returnvalue)) (`KismetMathLibrary.RandomFloatInRange` -30.0 30.0)))) "Undefined" "MultiplyWithRoot" null null))
  (`KismetSystemLibrary.Delay` (`self.FiringDelay`))
  (`self.ScatterShot`))

(event `OneShot`
  ; One Shot shot loop
  (`|SpawnActorFromClass` "/Game/MyContent/Blueprint/BP_Bullet.BP_Bullet_C" (`SceneComponent.GetSocketTransform` (`self.FiringPoint`) "None" "RTS_World") "Undefined" "MultiplyWithRoot" null null)
  (`KismetSystemLibrary.Delay` (`self.FiringDelay`))
  (`self.OneShot`))

(fn `UserConstructionScript`)