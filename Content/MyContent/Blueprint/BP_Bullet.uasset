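; BP_Bullet is a projectile actor that flies forward and damages the player's third-person character.
; BeginPlay caches the player pawn, and Tick offsets the actor along its forward vector by Speed each frame, without sweep or delta-time scaling.
; An overlap on SM_Bullet with the player calls DamageCharacter and destroys the bullet after a short delay.
; A LifeTime delay started from Tick also destroys it.
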(event `self.ReceiveBeginPlay`
  ; get player character
  (bind _asbp_third_person_character (cast `/Game/ThirdPerson/Blueprints/BP_ThirdPersonCharacter` (`GameplayStatics.GetPlayerPawn` 0)))
  (set `self.PlayerReference` _asbp_third_person_character))

(event `self.ReceiveTick`
  (params (DeltaSeconds :type "Float (single-precision)"))
  ; Bullet movement
  (`self.K2_AddActorWorldOffset` (* (`KismetMathLibrary.GetForwardVector` (`self.K2_GetActorRotation`)) (`self.Speed`)))
  (`KismetSystemLibrary.Delay` (`self.LifeTime`))
  (`self.K2_DestroyActor`))

(event `self.SM_Bullet.OnComponentBeginOverlap`
  (params (OverlappedComponent :type "PrimitiveComponent Object Reference") (OtherActor :type "Actor Object Reference") (OtherComp :type "PrimitiveComponent Object Reference") (OtherBodyIndex :type Integer) (bFromSweep :type Boolean) (SweepResult :type "HitResult Structure (by ref)"))
  (bind _playerreference (`self.PlayerReference`))
  ; on bullet hit player character
  (if (== OtherActor _playerreference)
    (`/Game/ThirdPerson/Blueprints/BP_ThirdPersonCharacter.DamageCharacter` _playerreference (`self.Damage`))
    (`KismetSystemLibrary.Delay` 0.2)
    (`self.K2_DestroyActor`)))

(fn `UserConstructionScript`)